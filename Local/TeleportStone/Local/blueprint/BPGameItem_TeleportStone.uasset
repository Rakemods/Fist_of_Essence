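; Teleport Stone game item that teleports the user to their owned bedroll, falling back to their bed.
; OnUseItem plays a portal effect and calls a server event, which resolves the bed by unique ID and checks ownership.
; The server consumes one stone before FindSpawnLocation capsule-sweeps hard-coded offsets around the bed for a clear spot.
; A failed search still costs the stone and shows "Cannot find bed"; P8 duplicates P7, leaving one corner untested.
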(event Custom|SRV_TeleportToBed
  (params (OtherActor :type Actor%20Object%20Reference))
  (bind _returnvalue (Class|GameItem|GetIntStat "StackSize"))
  (bind _returnvalue_2 (Class|GameItem|GetOwnerInventory))
  (bind _returnvalue_3 (Game|GetGameMode))
  (if (Ability|HasAuthority OtherActor)
    (bind _asbase_player_char (Utilities|Casting|CastToBasePlayerChar OtherActor))
    (Utilities|IsValid _returnvalue_3
      (:Is%20Valid
        ;[1 1 1] try BedrollID
        (bind _actor (Class|BaseGameModeInterface|GetActorbyUniqueIDInterface(Message) _returnvalue_3 (Variables|/Game/Characters/BasePlayerChar.BasePlayerChar_C|GetBedRollID _asbase_player_char)))
        (bind _output_get (Variables|Default|SetBedActor _actor))
        (Utilities|IsValid _output_get
          (:Is%20Valid
            (bind _asbuildable_base (Utilities|Casting|CastToBuildableBase _actor))
            (if (Class|BuildableBase|IsOwner _asbuildable_base _asbase_player_char false)
              (bind _asconan_player_controller (Utilities|Casting|CastToConanPlayerController (Pawn|GetController _asbase_player_char) :!label _label))
              (Utilities|FlowControl|Sequence
                (:then_0
                  ;[1 1 1] Consume item from item stack. If empty, remove item.
                  (if (<= _returnvalue 1)
                    (Class|ItemInventory|RemoveItem _returnvalue_2 (Class|ItemInventory|GetItemIndex _returnvalue_2 self))
                    (else
                      (Class|GameItem|SetIntStat "StackSize" (- _returnvalue 1) true))))
                (:then_1
                  ;[1 1 1] LootLog
                  (Class|ConanCharacter|ClientHUDLootNotification _asbase_player_char (Variables|Default|GetTemplateID) -1))
                (:then_2
                  (bind (_outlocation _success) (CallFunction|FindSpawnLocation (Variables|Default|GetBedActor)))
                  (if _success
                    (Class|ConanPlayerController|TeleportPlayerServer _asconan_player_controller _outlocation (Math|Rotator|MakeRotator 0.0 0.0 0.0) false false false false)
                    (Effects|SpawnEmitterAttached "/Game/Mods/Fist_of_Essence/InfinityBladeEffects/Effects/FX_Ability/Summon/P_Summon_Portal.P_Summon_Portal" (Variables|/Script/Engine.Character|GetMesh (stale EventOnUseItem _asbase_player_char)) "None")
                    (else
                      ;[1 1 1] no bed found
                      (Class|ConanCharacter|ClientHUDShowFIFO _asbase_player_char (Utilities|Text|MakeLiteralText "Cannot find bed") :!label _label_2)))))
              (else
                ;[1 1 1] if BedrollID invalid try BedID
                (bind _actor_2 (Class|BaseGameModeInterface|GetActorbyUniqueIDInterface(Message) _returnvalue_3 (Variables|/Game/Characters/BasePlayerChar.BasePlayerChar_C|GetBedID _asbase_player_char) :!label _label_3))
                (bind _output_get_2 (Variables|Default|SetBedActor _actor_2))
                (Utilities|IsValid _output_get_2
                  (:Is%20Valid
                    (bind _asbuildable_base_2 (Utilities|Casting|CastToBuildableBase _actor_2))
                    (if (Class|BuildableBase|IsOwner _asbuildable_base_2 _asbase_player_char false)
                      (goto _label)
                      (else
                        (goto _label_2))))
                  (:Is%20Not%20Valid
                    (goto _label_2))))))
          (:Is%20Not%20Valid
            (goto _label_3)))))))

(event EventOnUseItem
  (params (invokingCharacter :type Conan%20Character%20Object%20Reference))
  (bind _owneractor (Variables|Default|GetOwnerActor))
  (CallFunction|SRVTeleporttoBed _owneractor)
  (bind _asbase_player_char (Utilities|Casting|CastToBasePlayerChar (Components|GetOwner _owneractor)))
  (Effects|SpawnEmitterAttached "/Game/Mods/Fist_of_Essence/InfinityBladeEffects/Effects/FX_Ability/Summon/P_Summon_Portal.P_Summon_Portal" (Variables|/Script/Engine.Character|GetMesh _asbase_player_char) "None"))

(fn CanUseItem
  (params (invokingCharacter :type Conan%20Character%20Object%20Reference))
  (return true))

(fn FindSpawnLocation
  (params (BedActor :type Actor%20Object%20Reference))
  (bind _returnvalue (Actor|GetComponentsByClass BedActor "/Script/Engine.StaticMeshComponent"))
  (bind _array (Utilities|Array|MakeArray BedActor))
  (bind _item (Utilities|Array|Get(acopy) _returnvalue))
  (bind _origin (Collision|GetComponentBounds _item))
  ;[1 1 1] Sweep taken from "FunCombat_PlayerController->GetPlayerStart()"
  (Utilities|IsValid BedActor
    (:Is%20Valid
      (LocalVariables|SetOrigin (+ _origin "0.000000,0.000000,99.000000"))
      (LocalVariables|Setp1 (+ _origin "150.000000,0.000000,99.000000"))
      (LocalVariables|Setp2 (+ _origin "0,100.000000,99.000000"))
      (LocalVariables|Setp3 (+ _origin "-150.000000,0.000000,99.000000"))
      (LocalVariables|Setp4 (+ _origin "0,-100.000000,99.000000"))
      (LocalVariables|Setp5 (+ _origin "150.000000,100.000000,99.000000"))
      (LocalVariables|Setp6 (+ _origin "-150.000000,100.000000,99.000000"))
      (LocalVariables|Setp7 (+ _origin "-150.000000,-100.000000,99.000000"))
      (LocalVariables|Setp8 (+ _origin "-150.000000,-100.000000,99.000000"))
      (bind _returnvalue_2 (Class|KismetSystemLibrary|CapsuleTraceMulti (LocalVariables|GetOrigin) (LocalVariables|Getp1) 42.0 96.0 "TraceTypeQuery1" true _array "None" true))
      (if _returnvalue_2
        (bind _returnvalue_3 (Class|KismetSystemLibrary|CapsuleTraceMulti (LocalVariables|GetOrigin) (LocalVariables|Getp2) 42.0 96.0 "TraceTypeQuery1" true _array "None" true))
        (if _returnvalue_3
          (bind _returnvalue_4 (Class|KismetSystemLibrary|CapsuleTraceMulti (LocalVariables|GetOrigin) (LocalVariables|Getp3) 42.0 96.0 "TraceTypeQuery1" true _array "None" true))
          (if _returnvalue_4
            (bind _returnvalue_5 (Class|KismetSystemLibrary|CapsuleTraceMulti (LocalVariables|GetOrigin) (LocalVariables|Getp4) 42.0 96.0 "TraceTypeQuery1" true _array "None" true))
            (if _returnvalue_5
              (bind _returnvalue_6 (Class|KismetSystemLibrary|CapsuleTraceMulti (LocalVariables|GetOrigin) (LocalVariables|Getp5) 42.0 96.0 "TraceTypeQuery1" true _array "None" true))
              (if _returnvalue_6
                (bind _returnvalue_7 (Class|KismetSystemLibrary|CapsuleTraceMulti (LocalVariables|GetOrigin) (LocalVariables|Getp6) 42.0 96.0 "TraceTypeQuery1" true _array "None" true))
                (if _returnvalue_7
                  (bind _returnvalue_8 (Class|KismetSystemLibrary|CapsuleTraceMulti (LocalVariables|GetOrigin) (LocalVariables|Getp7) 42.0 96.0 "TraceTypeQuery1" true _array "None" true))
                  (if _returnvalue_8
                    (bind _returnvalue_9 (Class|KismetSystemLibrary|CapsuleTraceMulti (LocalVariables|GetOrigin) (LocalVariables|Getp8) 42.0 96.0 "TraceTypeQuery1" true _array "None" true))
                    (if _returnvalue_9
                      (return "0, 0, 0" false)
                      (else
                        (LocalVariables|SetSpawnLocation (LocalVariables|Getp8))))
                    (else
                      (LocalVariables|SetSpawnLocation (LocalVariables|Getp7))))
                  (else
                    (LocalVariables|SetSpawnLocation (LocalVariables|Getp6))))
                (else
                  (LocalVariables|SetSpawnLocation (LocalVariables|Getp5))))
              (else
                (LocalVariables|SetSpawnLocation (LocalVariables|Getp4))))
            (else
              (LocalVariables|SetSpawnLocation (LocalVariables|Getp3))))
          (else
            (LocalVariables|SetSpawnLocation (LocalVariables|Getp2))))
        (else
          (LocalVariables|SetSpawnLocation (LocalVariables|Getp1))))
      (return (LocalVariables|GetSpawnLocation) true))
    (:Is%20Not%20Valid
      (return "0, 0, 0" false))))