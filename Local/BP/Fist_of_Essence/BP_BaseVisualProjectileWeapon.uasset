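; Base visual actor for projectile weapons, holding the weapon's skeletal mesh and tracking a loaded projectile actor.
; It supplies the projectile launch location and rotation from the root component's Socket_Projectile, logging a debug message and falling back to the actor transform when the socket is missing.
; It also reads active ammunition from the owning weapon item and can destroy the loaded projectile.
; Equip and unequip handlers are empty.
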(event EventBeginPlay
  (|CallParentFunction))

(fn ConstructionScript
  (|CallParentFunction))

(fn HandleWeaponEquipped
  (params (GameItem :type Game%20Item%20Object%20Reference)))

(fn HandleWeaponUnEquipped
  (params (GameItem :type Game%20Item%20Object%20Reference)))

(fn DestroyLoadedProjectile
  (Utilities|IsValid (Variables|Default|GetLoadedProjectile)
    (:Is%20Valid
      (Actor|DestroyActor (Variables|Default|GetLoadedProjectile)))))

(fn GetAmmoID
  (return (Class|GameItem|GetIntStat (.Item (CallFunction|GetOwnerWeaponItem)) "ActiveAmmunition")))

(fn GetProjectileSocketLaunchLocation
  (bind _returnvalue (VehicleSound|GetRootComponent))
  (if (Transformation|DoesSocketExist _returnvalue "Socket_Projectile")
    (return (Transformation|GetSocketLocation _returnvalue "Socket_Projectile"))
    (else
      (Utilities|DebugPrintSimple (Utilities|String|ToString(Text) (Utilities|Text|FormatText "DEBUG: {char} using {wep} failed to get valid projectile socket location, returning the weapons location." (Utilities|Text|ToText(String) (Utilities|GetDisplayName (Variables|Default|GetCharacterOwner))) (Utilities|Text|ToText(String) (Utilities|GetDisplayName self)))) "INFOL_INFO2" "Combat"
        (:Output
          (return (Transformation|GetActorLocation self)))))))

(fn GetProjectileSocketLaunchRotation
  (bind _returnvalue (VehicleSound|GetRootComponent))
  (if (Transformation|DoesSocketExist _returnvalue "Socket_Projectile")
    (return (Transformation|GetSocketRotation _returnvalue "Socket_Projectile"))
    (else
      (Utilities|DebugPrintSimple (Utilities|String|ToString(Text) (Utilities|Text|FormatText "DEBUG: {char} using {wep} failed to get valid projectile socket rotation, returning the weapons rotation." (Utilities|Text|ToText(String) (Utilities|GetDisplayName (Variables|Default|GetCharacterOwner))) (Utilities|Text|ToText(String) (Utilities|GetDisplayName self)))) "INFOL_INFO2" "Combat"
        (:Output
          (return (Transformation|GetActorRotation self)))))))

(fn GetLoadedProjectile
  (return (Variables|Default|GetLoadedProjectile)))

(fn GetWeaponSkeletalMesh
  (return (Variables|Default|GetWeaponSkeletalMesh)))

(fn SetLoadedProjectile
  (params (ActorIn :type BP%20Base%20Projectile%20Object%20Reference))
  (bind _output_get (Variables|Default|SetLoadedProjectile ActorIn))
  (return _output_get))